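; Pombero boss enemy that chases the player, attacks with staff montages, and shows a boss widget while alive.
; On reaching the player it plays an attack montage, turns toward them during a timeline, then resumes the chase.
; PerformAttack collects characters through a dagger-socket capsule trace; FinishAttack damages them and applies the dealt damage to itself.
; When the game mode's obstacle list empties, it casts and has the obstacle manager spawn floor enemies.
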(event Custom|Follow%20Player
  (bind _returnvalue (Game|GetPlayerController 0))
  (bind _returnvalue_2 (Pawn|GetControlledPawn _returnvalue))
  (if (not (Variables|Default|GetIsAttacking))
    (AI|AIMoveTo self "0, 0, 0" (Game|Player|GetPlayerPawn 0) 5.0 true :!label _label
      (:OnSuccess
        (Animation|PlayAnimMontage "/Game/Toony_Tiny_RTS_Set_UE5/Animations/Units/Staff/Anim_staff_07_cast_A_Montage.Anim_staff_07_cast_A_Montage" 1.0 "None")
        (Variables|Default|SetIsAttacking true)
        (Timeline|Timeline PlayFromStart
          (:Update
            (Utilities|IsValid _returnvalue_2
              (:Is%20Valid
                (Transformation|SetActorRotation (Math|Rotator|FindLookatRotation (Transformation|GetActorLocation) (Transformation|GetActorLocation _returnvalue_2))))))
          (:Finished
            (goto _label)))))))

(event Custom|OnObstaclesChanged
  (params (Obstacles :type Array%20of%20BP%20Enemy%20Object%20References))
  (if (Utilities|Array|IsEmpty Obstacles)
    (Animation|PlayAnimMontage "/Game/Toony_Tiny_RTS_Set_UE5/Animations/Units/Staff/Anim_staff_07_cast_B_Montage.Anim_staff_07_cast_B_Montage" 1.0 "None")
    (Default|SpawnFloorEnemies (Variables|/Game/Blueprints/Enviroment/BP_GameplayGM.BP_GameplayGM_C|GetBPC_ObstacleManager (.AsBP%20Gameplay%20GM (Utilities|Casting|CastToBP_GameplayGM (Game|GetGameMode)))) false)))

(event Custom|FinishAttack
  (Audio|PlaySound2D "/Game/Sound/sword-sound-2-36274.sword-sound-2-36274" 1.0 1.0 0.15 0 0)
  (for _array_element (Variables|Default|GetAttackedCharacters)
    (bind _returnvalue (Game|Damage|ApplyDamage _array_element (Default|GetEffectiveDamage (Variables|Default|GetBPC_AttributesComponent)) 0 0))
    (Game|Damage|ApplyDamage self _returnvalue 0 0))
  (Utilities|Array|Clear (Variables|Default|GetAttackedCharacters)))

(event EventBeginPlay
  (|CallParentFunction)
  (EventDispatchers|BindEventtoOnSpawnedObstaclesChanged (Variables|/Game/Blueprints/Enviroment/BP_GameplayGM.BP_GameplayGM_C|GetBPC_ObstacleManager (.AsBP%20Gameplay%20GM (Utilities|Casting|CastToBP_GameplayGM (Game|GetGameMode)))) (delegate Custom|OnObstaclesChanged))
  (bind _returnvalue (UserInterface|CreateWidget "/Game/Blueprints/Widgets/WBP_Boss.WBP_Boss_C" (Game|GetPlayerController 0)))
  (bind _output_get (Variables|Default|SetWBP_Boss _returnvalue))
  (UserInterface|Viewport|AddtoViewport _output_get 0))

(event EventPerformAttack
  (bind _sm_w_dagger_a (Variables|Default|GetSM_w_dagger_A))
  (bind _returnvalue (Transformation|GetSocketLocation _sm_w_dagger_a "AttackSocket"))
  (bind _outhit (Class|KismetSystemLibrary|CapsuleTraceSingleforObjects _returnvalue _returnvalue 3e+01 45.0 (Utilities|Array|MakeArray "ObjectTypeQuery3") false 0 "None" true))
  (bind _ascharacter (Utilities|Casting|CastToCharacter (.HitActor (Collision|BreakHitResult _outhit))))
  (Utilities|Array|AddUnique (Variables|Default|GetAttackedCharacters) _ascharacter))

(event EventTick
  (params (DeltaSeconds :type Float%20%28single-precision%29))
  (CallFunction|FollowPlayer))

(event EventDestroyed
  (|CallParentFunction)
  (Widget|RemovefromParent (Variables|Default|GetWBP_Boss)))

(fn ConstructionScript
  (|CallParentFunction)
  (Components|SkinnedMesh|SetLeaderPoseComponent (Variables|Default|GetSK_Head_03d) (Variables|Character|GetMesh) false false))