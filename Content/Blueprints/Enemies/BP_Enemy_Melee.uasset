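; Melee enemy Blueprint for a wolf that chases the player, plays a bite montage and deals damage.
; Tick drives AIMoveTo until the first attack sets IsAttacking; thereafter, a timeline turns the wolf toward the player and restarts the move when finished.
; PerformAttack, not called within this graph, plays a sound, sphere-traces at the tongue socket with persistent debug drawing, and damages BP_MainCharacter using the attributes component's effective damage.
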(event Custom|Follow%20Player
  (bind _returnvalue (Game|GetPlayerController 0))
  (bind _returnvalue_2 (Pawn|GetControlledPawn _returnvalue))
  (if (not (Variables|Default|GetIsAttacking))
    (AI|AIMoveTo self "0, 0, 0" (Game|Player|GetPlayerPawn 0) 5.0 true :!label _label
      (:OnSuccess
        (Animation|PlayAnimMontage "/Game/PolyArtWolf/Animations/InPlace/Wolf_IP_Attack_Bite_Front_Montage.Wolf_IP_Attack_Bite_Front_Montage" 1.0 "None")
        (Variables|Default|SetIsAttacking true)
        (Timeline|Timeline PlayFromStart
          (:Update
            (Utilities|IsValid _returnvalue_2
              (:Is%20Valid
                (Transformation|SetActorRotation (Math|Rotator|FindLookatRotation (Transformation|GetActorLocation) (Transformation|GetActorLocation _returnvalue_2))))))
          (:Finished
            (goto _label)))))))

(event EventBeginPlay)

(event Collision|EventActorBeginOverlap
  (params (OtherActor :type Actor%20Object%20Reference)))

(event EventPerformAttack
  (bind _mesh (Variables|Character|GetMesh))
  (bind _returnvalue (Transformation|GetSocketLocation _mesh "TongueSocket"))
  (Audio|PlaySound2D "/Game/Sound/shortwolfattack.shortwolfattack" 0.2 1.0 0.0 0 0)
  (bind _outhit (Collision|SphereTraceForObjects _returnvalue _returnvalue 5e+01 (Utilities|Array|MakeArray "ObjectTypeQuery3") false 0 "Persistent"))
  (bind _asbp_main_character (Utilities|Casting|CastToBP_MainCharacter (.HitActor (Collision|BreakHitResult _outhit))))
  (Game|Damage|ApplyDamage _asbp_main_character (Default|GetEffectiveDamage (Variables|Default|GetBPC_AttributesComponent)) 0 0))

(event EventTick
  (params (DeltaSeconds :type Float%20%28single-precision%29))
  (CallFunction|FollowPlayer))

(fn ConstructionScript
  (|CallParentFunction))