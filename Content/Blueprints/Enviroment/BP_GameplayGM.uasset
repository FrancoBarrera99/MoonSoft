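; Gameplay game mode that runs a room-to-room floor system, spawning a random starting floor marked completed and restarting the player at the PlayerStart.
; SpawnFloor uses the door's diagonal tag to place a random neighboring floor, blends the camera to it and teleports the pawn to its facing door.
; The old floor is recorded by location in Floors and destroyed after a delay, while CompleteFloor flags the current one as cleared.
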(event EventBeginPlay
  (bind _returnvalue (Game|SpawnActorfromClass (CallFunction|GetRandomFloorClass true) (Math|Transform|MakeTransform "0, 0, 0") "Undefined" "MultiplyWithRoot" 0 0))
  (bind _output_get (Variables|Default|SetCurrentFloor _returnvalue))
  (Variables|/Game/Blueprints/Scenes/BP_Floor.BP_Floor_C|SetbIsCompleted _output_get true)
  (Game|Player|SetViewTargetwithBlend (Game|GetPlayerController 0) _output_get 0.0 "VTBlend_Linear" 0.0 false)
  (bind _returnvalue_2 (Actor|GetActorOfClass "/Script/Engine.PlayerStart"))
  (Class|GameModeBase|RestartPlayeratPlayerStart 0 _returnvalue_2))

(fn ConstructionScript)

(fn GetRandomFloorClass
  (params (bIsDefault :type Boolean))
  (bind _array (Utilities|Array|MakeArray "/Game/Blueprints/Scenes/BP_Floor_1.BP_Floor_1_C" "/Game/Blueprints/Scenes/BP_Floor_2.BP_Floor_2_C"))
  (bind _outitem (Utilities|Array|Random _array))
  (return (select bIsDefault _outitem _outitem)))

(fn SpawnFloor
  (params (InDoor :type BP%20Door%20Object%20Reference))
  (bind _returnvalue (Actor|GetParentActor InDoor))
  (bind _tags (Variables|/Script/Engine.Actor|GetTags InDoor))
  (bind _incrementalpositionvalue (LocalVariables|GetIncrementalPositionValue))
  (bind _returnvalue_2 (Transformation|GetActorLocation _returnvalue))
  (bind _output (Utilities|Array|Get(acopy) _tags))
  (bind _returnvalue_3 (* _incrementalpositionvalue -1.0))
  (Input|DisableInput (CallFunction|GetPawn) (Game|GetPlayerController 0))
  (switch name _output
    (:TopRight
      (LocalVariables|SetSpawnLocation (+ _returnvalue_2 (Math|Vector|MakeVector _incrementalpositionvalue _incrementalpositionvalue 0.0))))
    (:TopLeft
      (LocalVariables|SetSpawnLocation (+ _returnvalue_2 (Math|Vector|MakeVector _incrementalpositionvalue _returnvalue_3 0.0))))
    (:BottomRight
      (LocalVariables|SetSpawnLocation (+ _returnvalue_2 (Math|Vector|MakeVector _returnvalue_3 _incrementalpositionvalue 0.0))))
    (:BottomLeft
      (LocalVariables|SetSpawnLocation (+ _returnvalue_2 (Math|Vector|MakeVector _returnvalue_3 _returnvalue_3 0.0)))))
  (bind _returnvalue_4 (Game|SpawnActorfromClass (CallFunction|GetRandomFloorClass false) (Math|Transform|MakeTransform (LocalVariables|GetSpawnLocation)) "Undefined" "MultiplyWithRoot" 0 0))
  (Game|Player|SetViewTargetwithBlend (Game|GetPlayerController 0) _returnvalue_4 1.0 "VTBlend_Linear" 0.0 false)
  (bind _outdoor (Default|GetFacingDoor _returnvalue_4 _output))
  (Transformation|SetActorLocation (CallFunction|GetPawn) (Transformation|GetWorldLocation (Variables|/Game/Blueprints/Scenes/BP_Door.BP_Door_C|GetSpawnPoint _outdoor)) false false)
  (Input|EnableInput (CallFunction|GetPawn) (Game|GetPlayerController 0))
  (Utilities|Map|Add (Variables|Default|GetFloors) (Transformation|GetActorLocation (Variables|Default|GetCurrentFloor)) (Utilities|Struct|MakeF_FloorData (Utilities|GetClass (Variables|Default|GetCurrentFloor)) (Transformation|GetActorLocation (Variables|Default|GetCurrentFloor)) true))
  (Default|DelayedDestroy (Variables|Default|GetCurrentFloor))
  (Variables|Default|SetCurrentFloor _returnvalue_4))

(fn GetPawn
  (bind _asbp_third_person_character (Utilities|Casting|CastToBP_ThirdPersonCharacter (Pawn|GetControlledPawn (Game|GetPlayerController 0))))
  (return _asbp_third_person_character))

(fn CompleteFloor
  (Variables|/Game/Blueprints/Scenes/BP_Floor.BP_Floor_C|SetbIsCompleted (Variables|Default|GetCurrentFloor) true))