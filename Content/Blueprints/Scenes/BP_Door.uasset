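; BP_Door is a gate door that opens and closes by animated scaling, with an availability flag that other logic can read or set.
; ToggleDoor clears the flag, plays a timeline driving GateDoor's world scale, reverses it after a one-second pause, then restores the flag.
; SetAvailable also recolors three text renders green or red, whereas ToggleDoor writes the variable directly, leaving their color unchanged.
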(event Custom|ToggleDoor
  (Variables|Default|SetbAvailable false)
  (bind (_direction _scale) (Timeline|Timeline Play)
    (:Update
      (Transformation|SetWorldScale3D (Variables|Default|Getgate_door) (Math|Conversions|ToVector(Float) _scale)))
    (:Finished
      (switch Utilities|FlowControl|Switch|SwitchonETimelineDirection _direction
        (:Forward
          (Utilities|FlowControl|Delay 1.0)
          (Timeline|Timeline Reverse))
        (:Backward
          (Variables|Default|SetbAvailable true))))))

(fn ConstructionScript)

(fn IsAvailable
  (return (Variables|Default|GetbAvailable)))

(fn SetAvailable
  (params (bAvailable :type Boolean))
  (bind _output_get (Variables|Default|SetbAvailable bAvailable))
  (Rendering|Components|TextRender|SetTextRenderColor (Variables|Default|GetTextRender) (Math|Conversions|ToColor(LinearColor) (Math|Color|SelectColor "(R=0.014921,G=1.000000,B=0.000000,A=1.000000)" "(R=0.614583,G=0.000000,B=0.009863,A=1.000000)" _output_get))))