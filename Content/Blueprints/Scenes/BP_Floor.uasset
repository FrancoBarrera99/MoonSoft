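; BP_Floor is one floor of the level, built from floor data with tagged doors, optional bonus or final boss door, and a level label.
; Doors attach to tag-matched scene components, with tree meshes filling unused slots.
; Completion makes doors available and reveals the boss door.
; Character overlap on available doors asks the game mode's floor manager to spawn the next floor, or ends the game at the boss door.
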(event Custom|DelayedDestroy
  (Utilities|FlowControl|Delay 2.0)
  (for _array_element (Variables|Default|GetSpawnedDoors)
    (Actor|DestroyActor _array_element))
  (bind _bonus (Variables|Default|GetBonus)
    (:then
      (Actor|DestroyActor _bonus))
    (:else
      _))
  (Actor|DestroyActor))

(event Custom|SetFlootData
  (params (InFloorData :type F%20Floor%20Data%20Structure))
  (bind _output_get (Variables|Default|SetFloorData InFloorData))
  (CallFunction|SpawnDoors)
  (CallFunction|SetFloorLevel)
  (CallFunction|SetIsCompleted (.bIsCompleted (Utilities|Struct|BreakF_FloorData _output_get))))

(event Custom|SpawnDoors
  (bind _floordata (Variables|Default|GetFloorData))
  (bind _doortags (Utilities|Struct|BreakF_FloorData _floordata))
  (Utilities|FlowControl|Sequence
    (:then_0
      (if (Utilities|Array|ContainsItem _doortags "FinalBoss")
        ;[1 1 1] Spawn final boss door
        (bind _returnvalue (Game|SpawnActorfromClass "/Game/Blueprints/Scenes/BP_Door_End.BP_Door_End_C" (Math|Transform|MakeTransform "0, 0, 0") "Undefined" "MultiplyWithRoot" 0 0))
        (Transformation|AttachComponentToComponent _returnvalue (Variables|Default|GetDefaultSceneRoot) "None" "SnapToTarget" "SnapToTarget" "SnapToTarget" true)
        (Transformation|SetActorRelativeRotation _returnvalue "0.000000,90.000000,0.000000")
        (Variables|/Script/Engine.Actor|SetTags _returnvalue (.DoorTags (Utilities|Struct|BreakF_FloorData (Variables|Default|GetFloorData))))
        (Collision|BindEventtoOnActorBeginOverlap _returnvalue (delegate Custom|OnFinalDoorBeginOverlap))
        (Utilities|Array|Add (Variables|Default|GetSpawnedDoors) _returnvalue)
        (bind _output_get (Variables|Default|SetFinalDoor _returnvalue))
        (Rendering|SetActorHiddenInGame _output_get true)
        (Collision|SetActorEnableCollision _returnvalue false)
        (elif (Utilities|Array|ContainsItem _doortags "Bonus")
          (Utilities|FlowControl|Sequence
            (:then_0
              (bind _returnvalue_2 (Game|SpawnActorfromClass "/Game/Blueprints/Scenes/BP_GauchitoBonus.BP_GauchitoBonus_C" (Math|Transform|MakeTransform "0, 0, 0") "Undefined" "MultiplyWithRoot" 0 0))
              (Transformation|AttachComponentToComponent _returnvalue_2 (Variables|Default|GetDefaultSceneRoot) "None" "SnapToTarget" "SnapToTarget" "SnapToTarget" true)
              (Transformation|SetActorRelativeRotation _returnvalue_2 "0.000000,90.000000,0.000000")
              (Variables|Default|SetBonus _returnvalue_2))
            (:then_1
              ;[1 1 1] Spawn next floor doors
              (for _array_element (.DoorTags (Utilities|Struct|BreakF_FloorData (Variables|Default|GetFloorData))) :!label _label
                (bind _returnvalue_3 (Game|SpawnActorfromClass "/Game/Blueprints/Scenes/BP_Door.BP_Door_C" (Math|Transform|MakeTransform "0, 0, 0") "Undefined" "MultiplyWithRoot" 0 0))
                (Transformation|AttachComponentToComponent _returnvalue_3 (Utilities|Array|Get(acopy) (Actor|GetComponentsbyTag "/Script/Engine.SceneComponent" _array_element)) "None" "SnapToTarget" "SnapToTarget" "SnapToTarget" true)
                (Utilities|Array|RemoveItem (Variables|Default|GetAllDoorScenes) (Utilities|Array|Get(acopy) (Actor|GetComponentsbyTag "/Script/Engine.SceneComponent" _array_element)))
                (Transformation|SetActorRelativeLocation _returnvalue_3 "0.000000,60.000000,0.000000")
                (Variables|/Script/Engine.Actor|SetTags _returnvalue_3 (Utilities|Array|MakeArray _array_element))
                (Collision|BindEventtoOnActorBeginOverlap _returnvalue_3 (delegate Custom|OnDoorBeginOverlap))
                (Utilities|Array|Add (Variables|Default|GetSpawnedDoors) _returnvalue_3))))
          (else
            (goto _label)))))
    (:then_1
      (for _array_element_2 (Variables|Default|GetAllDoorScenes)
        (bind _returnvalue_4 (Game|AddComponentbyClass "/Script/Engine.StaticMeshComponent" false (Transformation|GetRelativeTransform _array_element_2)))
        (Components|StaticMesh|SetStaticMesh _returnvalue_4 "/Game/Assets/Custom/TreeDoor.TreeDoor")))))

(event Custom|OnFinalDoorBeginOverlap
  (params (OverlappedActor :type Actor%20Object%20Reference) (OtherActor :type Actor%20Object%20Reference))
  ;[1 1 1] Spawn final boss door
  (if (and (.bSuccess (Utilities|Casting|CastToCharacter OtherActor)) (.bIsCompleted (Utilities|Struct|BreakF_FloorData (Variables|Default|GetFloorData))))
    (bind _asbp_door (Utilities|Casting|CastToBP_Door OverlappedActor))
    (if (Default|IsAvailable _asbp_door)
      (bind _asbp_gameplay_gm (Utilities|Casting|CastToBP_GameplayGM (Game|GetGameMode)))
      (Default|EndGame _asbp_gameplay_gm))))

(event Custom|OnDoorBeginOverlap
  (params (OverlappedActor :type Actor%20Object%20Reference) (OtherActor :type Actor%20Object%20Reference))
  ;[1 1 1] Spawn next floor doors
  (if (and (.bSuccess (Utilities|Casting|CastToCharacter OtherActor)) (.bIsCompleted (Utilities|Struct|BreakF_FloorData (Variables|Default|GetFloorData))))
    (bind _asbp_door (Utilities|Casting|CastToBP_Door OverlappedActor))
    (if (Default|IsAvailable _asbp_door)
      (bind _asbp_gameplay_gm (Utilities|Casting|CastToBP_GameplayGM (Game|GetGameMode)))
      (Default|SpawnFloor (Variables|/Game/Blueprints/Enviroment/BP_GameplayGM.BP_GameplayGM_C|GetBPC_FloorManager _asbp_gameplay_gm) (Transformation|GetActorLocation) (Utilities|Array|Get(acopy) (Variables|/Script/Engine.Actor|GetTags OverlappedActor)))
      (Default|ToggleDoor _asbp_door))))

(fn ConstructionScript
  (Variables|Default|SetAllDoorScenes (Utilities|Array|MakeArray (Variables|Default|GetDoorScene) (Variables|Default|GetDoorScene2) (Variables|Default|GetDoorScene3) (Variables|Default|GetDoorScene4))))

(fn GetFacingDoor
  (params (InPreviousDoorTag :type Name))
  (bind _array_element (Utilities|Array|ForEachLoopwithBreak (Actor|GetAttachedActors true false) :!label _label)
    (:LoopBody
      (if (and (.bSuccess (Utilities|Casting|CastToBP_Door _array_element)) (Utilities|Array|ContainsItem (Variables|/Script/Engine.Actor|GetTags _array_element) (CallFunction|GetOppositeDoorTag InPreviousDoorTag)))
        (LocalVariables|SetOutDootVar (.AsBP%20Door (Utilities|Casting|CastToBP_Door _array_element)))
        (goto _label Break)))
    (:Completed
      (Utilities|IsValid (LocalVariables|GetOutDootVar)
        (:Is%20Valid
          (return (LocalVariables|GetOutDootVar)))
        (:Is%20Not%20Valid
          (return (Variables|Default|GetFinalDoor)))))))

(fn SetIsCompleted
  (params (bIsCompleted :type Boolean))
  (bind _finaldoor (Variables|Default|GetFinalDoor))
  (Utilities|Struct|SetmembersinF_FloorData (Variables|Default|GetFloorData) bIsCompleted)
  (for _array_element (Variables|Default|GetSpawnedDoors)
    (Default|SetAvailable _array_element bIsCompleted))
  (if (and bIsCompleted (Utilities|IsValid _finaldoor))
    (Rendering|SetActorHiddenInGame _finaldoor false)
    (Collision|SetActorEnableCollision _finaldoor true)))

(fn IsCompleted
  (return (.bIsCompleted (Utilities|Struct|BreakF_FloorData (Variables|Default|GetFloorData)))))

(fn GetFloorData
  (return (Variables|Default|GetFloorData)))

(fn SetFloorLevel
  (bind _floordata (Variables|Default|GetFloorData))
  (bind (_class _position _biscompleted _level) (Utilities|Struct|BreakF_FloorData _floordata))
  (bind (_x _y) (Math|Vector|BreakVector _position))
  (Rendering|Components|TextRender|SetText (Variables|Default|GetFloorLevel) (Utilities|Text|ToText(String) (Utilities|String|Append "Level: " (Utilities|String|ToString(Integer) _level) " 
{" (Utilities|String|ToString(Float) _x) "," (Utilities|String|ToString(Float) _y) "}"))))

(fn GetObstacleSpawnTransform
  (return (Math|Transform|SelectTransform (Transformation|GetWorldTransform (Variables|Default|GetObstacleSpawnPoint1)) (Transformation|GetWorldTransform (Variables|Default|GetObstacleSpawnPoint2)) (Math|Random|RandomBool))))