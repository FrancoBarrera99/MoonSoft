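; BP_GauchitoBonus is a one-time bonus trigger that opens the bonus GUI when the main character touches it.
; Its capsule overlap checks that the bonus is unused and that the game mode's floor manager reports the current floor as not completed.
; It then asks the player's HUD to show the bonus GUI and marks itself consumed, leaving any reward logic outside this Blueprint.
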(event OnComponentBeginOverlap(Capsule)
  (params (OverlappedComponent :type Primitive%20Component%20Object%20Reference) (OtherActor :type Actor%20Object%20Reference) (OtherComp :type Primitive%20Component%20Object%20Reference) (OtherBodyIndex :type Integer) (bFromSweep :type Boolean) (SweepResult :type Hit%20Result%20Structure%20%28by%20ref%29))
  (if (Math|Boolean|ANDBoolean (.bSuccess (Utilities|Casting|CastToBP_MainCharacter OtherActor)) (not (Variables|Default|GetbBonusConsumed)) (not (Default|IsCompleted (Variables|/Game/Blueprints/Components/BPC_FloorManager.BPC_FloorManager_C|GetCurrentFloor (Variables|/Game/Blueprints/Enviroment/BP_GameplayGM.BP_GameplayGM_C|GetBPC_FloorManager (.AsBP%20Gameplay%20GM (Utilities|Casting|CastToBP_GameplayGM (Game|GetGameMode))))))))
    (bind _asbp_hud (Utilities|Casting|CastToBP_HUD (HUD|GetHUD (Game|GetPlayerController 0))))
    (Default|ShowBonusGUI _asbp_hud)
    (Variables|Default|SetbBonusConsumed true)))

(fn ConstructionScript)