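; Floor manager component that procedurally builds a dungeon-like grid of connected floors as the player passes through diagonal doors.
; Floor data is cached by location, so revisits respawn the same layout, while new floors gain a level and random doors including one back.
; Past level four, a chance roll yields a final-boss floor with only a middle escape door.
; Transitions blend the camera, teleport the pawn and delay-destroy the previous floor; invalid directions spawn the default floor.
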(fn SpawnFloor
  (params (CurrentPosition :type Vector) (CurrentDoorTag :type Name))
  (bind (_calculatedlocation _bvaliddirection) (CallFunction|CalculateDirectionalLocation CurrentPosition CurrentDoorTag))
  (if _bvaliddirection
    (LocalVariables|SetSpawnLocation _calculatedlocation)
    (if (.ReturnValue (Utilities|Map|Find (Variables|Default|GetFloors) (LocalVariables|GetSpawnLocation)))
      (LocalVariables|SetSpawnFloorData (.Value (Utilities|Map|Find (Variables|Default|GetFloors) (LocalVariables|GetSpawnLocation))))
      (else
        (bind _output_get (LocalVariables|SetSpawnFloorData (Utilities|Struct|MakeF_FloorData 0 (LocalVariables|GetSpawnLocation) false (+ (.Level (Utilities|Struct|BreakF_FloorData (Default|GetFloorData (Variables|Default|GetCurrentFloor)))) 1) (CallFunction|GetRandomDoorTags (CallFunction|GetOppositeDoorTag CurrentDoorTag)))))
        (Utilities|Map|Add (Variables|Default|GetFloors) (LocalVariables|GetSpawnLocation) _output_get)
        (Variables|Default|SetCurrentGameLevel (+ (.Level (Utilities|Struct|BreakF_FloorData (Default|GetFloorData (Variables|Default|GetCurrentFloor)))) 1))))
    (bind _custom_floor (CallFunction|SpawnCustomizedFloor (LocalVariables|GetSpawnFloorData)))
    (Game|Player|SetViewTargetwithBlend (Game|GetPlayerController 0) _custom_floor 2.0 "VTBlend_Linear" 0.0 false)
    (bind _outdoor (Default|GetFacingDoor _custom_floor CurrentDoorTag))
    (Default|ToggleDoor _outdoor)
    (Transformation|SetActorLocation (CallFunction|GetPawn) (Transformation|GetWorldLocation (Variables|/Game/Blueprints/Scenes/BP_Door.BP_Door_C|GetSpawnPoint _outdoor)) false true)
    (Default|DelayedDestroy (Variables|Default|GetCurrentFloor))
    (Variables|Default|SetCurrentFloor _custom_floor)
    (else
      (CallFunction|SpawnDefaultFloor))))

(fn CompleteFloor
  (Default|SetIsCompleted (Variables|Default|GetCurrentFloor) true))

(fn GetPawn
  (bind _asbp_third_person_character (Utilities|Casting|CastToBP_ThirdPersonCharacter (Pawn|GetControlledPawn (Game|GetPlayerController 0))))
  (return _asbp_third_person_character))

(fn SpawnDefaultFloor
  (bind _outgamemode (CallFunction|GetOwnerGameMode))
  (bind _array (Utilities|Array|MakeArray "TopLeft"))
  (bind _f_floordata (Utilities|Struct|MakeF_FloorData "/Game/Blueprints/Scenes/BP_Floor_Default.BP_Floor_Default_C" "0.000000,0.000000,0.000000" true 1 _array))
  (bind _returnvalue (Game|SpawnActorfromClass "/Game/Blueprints/Scenes/BP_Floor.BP_Floor_C" (Math|Transform|MakeTransform "0, 0, 0") "Undefined" "MultiplyWithRoot" 0 0))
  (bind _output_get (Variables|Default|SetCurrentFloor _returnvalue))
  (Default|SetFlootData _output_get _f_floordata)
  (Utilities|Map|Add :TargetMap (Variables|Default|GetFloors) :Value _f_floordata)
  (Game|Player|SetViewTargetwithBlend (Game|GetPlayerController 0) _output_get 0.0 "VTBlend_Linear" 0.0 false)
  (bind _returnvalue_2 (Actor|GetActorOfClass "/Script/Engine.PlayerStart"))
  (Utilities|IsValid _outgamemode
    (:Is%20Valid
      (Class|GameModeBase|RestartPlayeratPlayerStart _outgamemode 0 _returnvalue_2))))

(fn GetOwnerGameMode
  (bind _asbp_gameplay_gm (Utilities|Casting|CastToBP_GameplayGM (Game|GetGameMode)))
  (return _asbp_gameplay_gm))

(fn SpawnCustomizedFloor
  (params (FloorData :type F%20Floor%20Data%20Structure))
  (bind _returnvalue (Game|SpawnActorfromClass "/Game/Blueprints/Scenes/BP_Floor.BP_Floor_C" (Math|Transform|MakeTransform (.Position (Utilities|Struct|BreakF_FloorData FloorData))) "Undefined" "MultiplyWithRoot" 0 0))
  (Default|SetFlootData _returnvalue FloorData)
  (return _returnvalue))

(fn GetNextFloorTags)

(fn GetRandomDoorTags
  (params (MandatoryTag :type Name))
  (bind _directiontags (LocalVariables|GetDirectionTags))
  (bind _returnvalue (Utilities|Array|Length _directiontags))
  (bind _returnvalue_2 (- _returnvalue 1))
  (bind _returnvalue_3 (Math|Random|RandomIntegerinRange 0 _returnvalue_2))
  (bind _output (Utilities|Array|Get(acopy) _directiontags _returnvalue_3))
  (if (and (> (Variables|Default|GetCurrentGameLevel) 4) (<= (Math|Random|RandomFloatinRange 0.0 1.0) (Variables|Default|GetFinalBossProbability)))
    ;[1 1 1] If there's a final boss, create a middle door to scape once the floor is completed
    (Utilities|Array|Add (LocalVariables|GetOutTags) "Middle")
    (return (LocalVariables|GetOutTags))
    (else
      ;[1 1 1] Add mandatory previous floor door tag
      (Utilities|Array|Add (LocalVariables|GetOutTags) MandatoryTag)
      (Utilities|Array|RemoveItem (LocalVariables|GetDirectionTags) MandatoryTag)
      ;[1 1 1] Add random mandatory next door tag
      (Utilities|Array|Add (LocalVariables|GetOutTags) _output)
      (Utilities|Array|RemoveItem (LocalVariables|GetDirectionTags) _output)
      (for _array_element (LocalVariables|GetDirectionTags)
        (if (<= (Math|Random|RandomFloatinRange 0.0 1.0) (LocalVariables|GetRandomDoorPercentage))
          (Utilities|Array|Add (LocalVariables|GetOutTags) _array_element)))
      (return (LocalVariables|GetOutTags)))))

(fn CalculateDirectionalLocation
  (params (CurrentLocation :type Vector) (DirectionTag :type Name))
  (bind _incrementalpositionvalue (LocalVariables|GetIncrementalPositionValue))
  (bind _returnvalue (* _incrementalpositionvalue -1.0))
  (switch name DirectionTag
    (:Default
      (LocalVariables|SetbValid false))
    (:TopRight
      (LocalVariables|SetOutLocation (+ CurrentLocation (Math|Vector|MakeVector _incrementalpositionvalue _incrementalpositionvalue 0.0)))
      (LocalVariables|SetbValid true :!label _label))
    (:TopLeft
      (LocalVariables|SetOutLocation (+ CurrentLocation (Math|Vector|MakeVector _incrementalpositionvalue _returnvalue 0.0)))
      (goto _label))
    (:BottomRight
      (LocalVariables|SetOutLocation (+ CurrentLocation (Math|Vector|MakeVector _returnvalue _incrementalpositionvalue 0.0)))
      (goto _label))
    (:BottomLeft
      (LocalVariables|SetOutLocation (+ CurrentLocation (Math|Vector|MakeVector _returnvalue _returnvalue 0.0)))
      (goto _label)))
  (return (LocalVariables|GetOutLocation) (LocalVariables|GetbValid)))