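; Component that computes a level difficulty value from the current game level tracked by the gameplay game mode's floor manager.
; GetLevelDifficulty applies a logistic S-curve shaped by max bound, growth rate and inflection point, then divides the result by 100.
; On BeginPlay it binds to the floor manager's floor-spawned event, where it only prints the current difficulty.
; A getter also exposes the maximum difficulty bound.
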(event Custom|CustomEvent
  (params (FloorData :type F%20Floor%20Data%20Structure))
  (Development|PrintString (Utilities|String|ToString(Float) (CallFunction|GetLevelDifficulty))))

(event EventBeginPlay
  (bind _asbp_gameplay_gm (Utilities|Casting|CastToBP_GameplayGM (Game|GetGameMode)))
  (EventDispatchers|BindEventtoOnFloorSpawned (Variables|/Game/Blueprints/Enviroment/BP_GameplayGM.BP_GameplayGM_C|GetBPC_FloorManager _asbp_gameplay_gm) (delegate Custom|CustomEvent)))

(fn GetLevelDifficulty
  (bind _asbp_gameplay_gm (Utilities|Casting|CastToBP_GameplayGM (Game|GetGameMode)))
  (return (/ (/ (Variables|Default|GetMaxDifficultyBound) (+ 1.0 (Class|KismetMathLibrary|Exp (* (* (Variables|Default|GetDifficultyGrowthRate) -1.0) (- (Variables|/Game/Blueprints/Components/BPC_FloorManager.BPC_FloorManager_C|GetCurrentGameLevel (Variables|/Game/Blueprints/Enviroment/BP_GameplayGM.BP_GameplayGM_C|GetBPC_FloorManager _asbp_gameplay_gm)) (Variables|Default|GetDifficultyInflectionPoint)))))) 1e+02)))

(fn GetMaxDifficultyBound
  (return (Variables|Default|GetMaxDifficultyBound)))