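; BPC_AttributesComponent is a component that manages a character's attributes and handles damage and death.
; On BeginPlay it binds to its Character owner's any-damage event, reduces incoming damage by Armor, and clamps the resulting Health.
; It broadcasts OnAttributesUpdated after each hit and destroys the owner when Health reaches zero.
; GetEffectiveDamage returns BaseDamage scaled up by Strength.
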(event Custom|On%20Take%20Any%20Damage
  (params (DamagedActor :type Actor%20Object%20Reference) (Damage :type Float%20%28single-precision%29) (DamageType :type Damage%20Type%20Object%20Reference) (InstigatedBy :type Controller%20Object%20Reference) (DamageCauser :type Actor%20Object%20Reference))
  (bind _characterattributes (Variables|Default|GetCharacterAttributes))
  (bind _returnvalue (/ (.armor _characterattributes) 1e+02))
  (bind _returnvalue_2 (+ 1.0 _returnvalue))
  (bind _returnvalue_3 (/ Damage _returnvalue_2))
  (bind _returnvalue_4 (- (.health _characterattributes) _returnvalue_3))
  (bind _returnvalue_5 (Math|Float|Clamp(Float) _returnvalue_4 0.0 1e+02))
  (bind _structout (Utilities|Struct|SetmembersinF_CharacterAttributesData (Variables|Default|GetCharacterAttributes) _returnvalue_5))
  (Default|CallOnAttributesUpdated _structout)
  (if (== _returnvalue_5 0.0)
    (Actor|DestroyActor (Components|GetOwner))))

(event EventBeginPlay
  (bind _ascharacter (Utilities|Casting|CastToCharacter (Components|GetOwner)))
  (EventDispatchers|BindEventtoOnTakeAnyDamage _ascharacter (delegate Custom|On%20Take%20Any%20Damage)))

(fn GetEffectiveDamage
  (bind _characterattributes (Variables|Default|GetCharacterAttributes))
  (return (* (.basedamage _characterattributes) (+ 1.0 (/ (.strength _characterattributes) 1e+02)))))