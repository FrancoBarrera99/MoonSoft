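; Game mode component that populates each uncompleted floor with enemy obstacles and completes the floor once all are destroyed.
; On the floor manager's spawn event, it loops from 2 to the floor's level, placing random melee or ranged enemies at floor-provided transforms.
; A counter tracks destruction events and calls CompleteFloor at zero; the check runs only on destruction, so floors spawning no enemies are not completed here.
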(event Custom|OnFloorSpawned
  (params (FloorData :type F%20Floor%20Data%20Structure))
  (if (not (.bIsCompleted (Utilities|Struct|BreakF_FloorData FloorData)))
    (CallFunction|SpawnFloorObstacles)))

(event Custom|SpawnFloorObstacles
  (bind _bp_gameplay_gm (Variables|Default|GetBP%20Gameplay%20GM))
  (bind _bpc_floormanager (Variables|/Game/Blueprints/Enviroment/BP_GameplayGM.BP_GameplayGM_C|GetBPC_FloorManager _bp_gameplay_gm))
  (bind _currentfloor (Variables|/Game/Blueprints/Components/BPC_FloorManager.BPC_FloorManager_C|GetCurrentFloor _bpc_floormanager))
  (for _index (range 2 (.Level (Utilities|Struct|BreakF_FloorData (Default|GetFloorData _currentfloor))))
    (bind _transform (Default|GetObstacleSpawnTransform _currentfloor))
    (bind _returnvalue (Game|SpawnActorfromClass (CallFunction|GetRandomEnemyClass) _transform "Undefined" "MultiplyWithRoot" 0 0))
    (Game|BindEventtoOnDestroyed _returnvalue (delegate Custom|OnObstacleDestroyed))
    (Math|Integer|IncrementInt (Variables|Default|GetSpawnedObstacles))))

(event Custom|OnObstacleDestroyed
  (params (DestroyedActor :type Actor%20Object%20Reference))
  (Math|Integer|DecrementInt (Variables|Default|GetSpawnedObstacles)
    (:%20%20
      (CallFunction|CheckFloorRemainingObstacles))))

(event EventBeginPlay
  (bind _asbp_gameplay_gm (Utilities|Casting|CastToBP_GameplayGM (Components|GetOwner)))
  (bind _output_get (Variables|Default|SetBP%20Gameplay%20GM _asbp_gameplay_gm))
  (EventDispatchers|BindEventtoOnFloorSpawned (Variables|/Game/Blueprints/Enviroment/BP_GameplayGM.BP_GameplayGM_C|GetBPC_FloorManager _output_get) (delegate Custom|OnFloorSpawned)))

(fn CheckFloorRemainingObstacles
  (if (< (Variables|Default|GetSpawnedObstacles) 1)
    (Default|CompleteFloor (Variables|/Game/Blueprints/Enviroment/BP_GameplayGM.BP_GameplayGM_C|GetBPC_FloorManager (Variables|Default|GetBP%20Gameplay%20GM)))))

(fn GetRandomEnemyClass
  (return (Utilities|Select :Index (Math|Random|RandomIntegerinRange 0 1) :Option%200 "/Game/Blueprints/Enemies/BP_Enemy_Melee.BP_Enemy_Melee_C" :Option%201 "/Game/Blueprints/Enemies/BP_Enemy_Ranged.BP_Enemy_Ranged_C")))